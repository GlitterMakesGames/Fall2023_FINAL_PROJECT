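; Player character Blueprint with jumping, camera-relative movement and a line-trace gun.
; Turn input yaws the Cube and SpringArm components directly by the raw axis value, rather than using controller yaw.
; Fire traces on the Visibility channel along the GunNozzle's up vector and draws a red debug line.
; A hit on a Target actor tagged "ShootThis" calls its ToggleMaterial.
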(event `InputAction|Jump`
  (params (Key :type "Key Structure"))
  (:`Pressed`
    (`self.Jump`)))

(event `InputAxis|MoveForward`
  (params (AxisValue :type "Float (single-precision)"))
  (`self.AddMovementInput` (`KismetMathLibrary.GetForwardVector` (`SceneComponent.K2_GetComponentRotation` (`self.Camera`))) AxisValue))

(event `InputAxis|MoveRight`
  (params (AxisValue :type "Float (single-precision)"))
  (`self.AddMovementInput` (`KismetMathLibrary.GetRightVector` (`SceneComponent.K2_GetComponentRotation` (`self.Camera`))) AxisValue))

(event `InputAxis|Turn`
  (params (AxisValue :type "Float (single-precision)"))
  (bind _returnvalue (`KismetMathLibrary.MakeRotator` 0.0 0.0 AxisValue))
  (`SceneComponent.K2_AddRelativeRotation` (`self.Cube`) _returnvalue false false)
  (`SceneComponent.K2_AddRelativeRotation` (`self.SpringArm`) _returnvalue false false))

(event `InputAction|Fire`
  (params (Key :type "Key Structure"))
  (bind _gun_nozzle (`self.Gun Nozzle`))
  (bind _returnvalue (`SceneComponent.K2_GetComponentLocation` _gun_nozzle))
  (bind _returnvalue_2 (+ _returnvalue (* (`KismetMathLibrary.GetUpVector` (`SceneComponent.K2_GetComponentRotation` _gun_nozzle)) (`self.Distance`))))
  (:`Pressed`
    (bind (_outhit _returnvalue_3) (`KismetSystemLibrary.LineTraceSingle` :`Start` _returnvalue :`End` _returnvalue_2 :`TraceChannel` "TraceTypeQuery1" :`DrawTime` 1.0))
    (`KismetSystemLibrary.DrawDebugLine` (`SceneComponent.K2_GetComponentLocation` (`self.Gun Nozzle`)) _returnvalue_2 (struct :`R` 1.0 :`A` 1.0) 1.0 1.0)
    (if _returnvalue_3
      (bind (_bblockinghit _binitialoverlap _time _distance _location _impactpoint _normal _impactnormal _physmat _hitactor) (`GameplayStatics.BreakHitResult` _outhit))
      (if (`self.ActorHasTag` _hitactor "ShootThis")
        (bind _astarget (cast `Target` _hitactor))
        (`Target.ToggleMaterial` _astarget)))))

(fn `UserConstructionScript`)